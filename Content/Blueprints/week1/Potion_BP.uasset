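; Potion_BP is a pickup actor for health and mana potions that the main character collects by interacting with it.
; The construction script creates a dynamic instance of Potion_MI on the static mesh and tints its Color parameter red or blue according to PotionType.
; On HandleInteraction it passes the type to the character's AddPotion and destroys itself only if that call succeeds.
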(event EventHandleInteraction
  (bind _canpick (Default|AddPotion (Variables|Default|GetMainCharacterRef) (Variables|Default|GetPotionType)))
  (if _canpick
    (Actor|DestroyActor)))

(fn ConstructionScript
  (bind _returnvalue (Rendering|Material|CreateDynamicMaterialInstance (Variables|Default|GetStaticMesh) 0 "/Game/Blueprints/week1/Potion_MI.Potion_MI" "None" :!class /Script/Engine.PrimitiveComponent))
  (Rendering|Material|SetVectorParameterValue _returnvalue "Color" (Utilities|Select :Index (Variables|Default|GetPotionType) :NewEnumerator0 "(R=1.000000,G=0.000000,B=0.057817,A=1.000000)" :NewEnumerator1 "(R=0.000000,G=0.403484,B=1.000000,A=1.000000)") :!class /Script/Engine.MaterialInstanceDynamic))