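; InteractableObject_BP is a base interactable actor that responds to the player's interaction while the ThirdPersonCharacter is within its sphere.
; On BeginPlay it caches a reference to the player character.
; Entering the sphere binds its HandleInteraction event to the character's interaction dispatcher, and leaving unbinds all events from that dispatcher, including any other object's binding.
; HandleInteraction is empty here.
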(event OnComponentBeginOverlap(Sphere)
  (params (OverlappedComponent :type Primitive%20Component%20Object%20Reference) (OtherActor :type Actor%20Object%20Reference) (OtherComp :type Primitive%20Component%20Object%20Reference) (OtherBodyIndex :type Integer) (bFromSweep :type Boolean) (SweepResult :type Hit%20Result%20Structure%20%28by%20ref%29))
  (bind _asthird_person_character (Utilities|Casting|CastToThirdPersonCharacter OtherActor))
  (EventDispatchers|BindEventtoHandleInteraction _asthird_person_character (delegate Custom|HandleInteraction)))

(event OnComponentEndOverlap(Sphere)
  (params (OverlappedComponent :type Primitive%20Component%20Object%20Reference) (OtherActor :type Actor%20Object%20Reference) (OtherComp :type Primitive%20Component%20Object%20Reference) (OtherBodyIndex :type Integer))
  (bind _asthird_person_character (Utilities|Casting|CastToThirdPersonCharacter OtherActor))
  (EventDispatchers|UnbindallEventsfromHandleInteraction _asthird_person_character))

(event Custom|HandleInteraction)

(event Custom|SpotMainCharacter
  (bind _asthird_person_character (Utilities|Casting|CastToThirdPersonCharacter (Game|GetPlayerCharacter 0)))
  (Variables|Default|SetMainCharacterRef _asthird_person_character))

(event EventBeginPlay
  (CallFunction|SpotMainCharacter))

(fn ConstructionScript)