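; Enemy actor that hurts the third-person player on contact and can be damaged by stomping, in Mario style.
; Sphere overlap shrinks a big player or deducts health, while Box overlap bounces the player up and damages the enemy, destroying it with an explosion sound at zero health.
; A widget health bar turns toward the player camera every tick.
; BeginPlay starts a looping timer, and SetBlock briefly enables a visible, collidable Block.
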(event OnComponentBeginOverlap(Sphere)
  (params (OverlappedComponent :type Primitive%20Component%20Object%20Reference) (OtherActor :type Actor%20Object%20Reference) (OtherComp :type Primitive%20Component%20Object%20Reference) (OtherBodyIndex :type Integer) (bFromSweep :type Boolean) (SweepResult :type Hit%20Result%20Structure%20%28by%20ref%29))
  (bind _asthird_person_character (Utilities|Casting|CastToThirdPersonCharacter OtherActor))
  (if (Variables|/Game/ThirdPersonBP/Blueprints/ThirdPersonCharacter.ThirdPersonCharacter_C|GetisBig _asthird_person_character)
    (Transformation|SetActorScale3D _asthird_person_character "1.000000,1.000000,1.000000")
    (Variables|/Game/ThirdPersonBP/Blueprints/ThirdPersonCharacter.ThirdPersonCharacter_C|SetisBig _asthird_person_character false)
    (else
      (Default|ChangeHealth _asthird_person_character "NewEnumerator1" -5e+01)
      (Default|RestoreHealth _asthird_person_character))))

(event OnComponentBeginOverlap(Box)
  (params (OverlappedComponent :type Primitive%20Component%20Object%20Reference) (OtherActor :type Actor%20Object%20Reference) (OtherComp :type Primitive%20Component%20Object%20Reference) (OtherBodyIndex :type Integer) (bFromSweep :type Boolean) (SweepResult :type Hit%20Result%20Structure%20%28by%20ref%29))
  (bind _asthird_person_character (Utilities|Casting|CastToThirdPersonCharacter OtherActor))
  (Character|LaunchCharacter _asthird_person_character "0, 0,400.000000" false true)
  (CallFunction|ChangeEnemyHealth 5e+01))

(event Custom|SetBlock
  (bind _block (Variables|Default|GetBlock))
  (bind _block_2 (Variables|Default|GetBlock))
  (Rendering|SetVisibility _block_2 true false)
  (Collision|SetCollisionEnabled _block_2 "QueryAndPhysics")
  (Utilities|FlowControl|Delay 3.0)
  (Rendering|SetVisibility _block false false)
  (Collision|SetCollisionEnabled _block "NoCollision"))

(event EventBeginPlay
  (bind _returnvalue (UserInterface|CreateWidget "/Game/Blueprints/week2/HealthBar_UI.HealthBar_UI_C" 0 self))
  (UserInterface|SetWidget (Variables|Default|GetHealthBar) _returnvalue)
  (Utilities|Time|SetTimerbyEvent (EventDispatchers|CreateEvent :!event Custom|SetBlock) 5.0 true)
  (bind _asthird_person_character (Utilities|Casting|CastToThirdPersonCharacter (Game|GetPlayerCharacter 0)))
  (Variables|Default|SetMainCharRef _asthird_person_character))

(event EventTick
  (params (DeltaSeconds :type Float%20%28single-precision%29))
  (Transformation|SetWorldRotation (Variables|Default|GetHealthBar) (Math|Rotator|FindLookatRotation (Transformation|GetActorLocation) (Transformation|GetWorldLocation (Variables|/Game/ThirdPersonBP/Blueprints/ThirdPersonCharacter.ThirdPersonCharacter_C|GetFollowCamera (Variables|Default|GetMainCharRef)))) false false))

(fn ConstructionScript)

(fn ChangeEnemyHealth
  (params (Points :type Float%20%28single-precision%29))
  (bind _output_get (Variables|Default|SetHealth (- (Variables|Default|GetHealth) Points)))
  (if (not (> _output_get 0.0))
    (Actor|DestroyActor)
    (Audio|PlaySound2D "/Game/Blueprints/week2/explosion.explosion" 1.0 1.0 0.0 0 0)))